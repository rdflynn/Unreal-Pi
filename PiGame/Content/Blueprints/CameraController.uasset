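; CameraController is an actor that follows a Target actor's position and rotation every Tick.
; It moves by a MoveSpeed fraction of the world-space gap, applied as a local offset without DeltaSeconds scaling or sweep.
; Rotation lerps from the Target's rotation toward its own by DeltaSeconds times RotateSpeed, so smaller alphas stay closer to the Target's rotation.
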(event `self.ReceiveTick`
  (params (DeltaSeconds :type "Float (single-precision)"))
  (`self.K2_AddActorLocalOffset` (* (- (`self.K2_GetActorLocation` (`self.target`)) (`self.K2_GetActorLocation`)) (`self.moveSpeed`)))
  (`self.K2_SetActorRotation` (`KismetMathLibrary.RLerp` (`self.K2_GetActorRotation` (`self.target`)) (`self.K2_GetActorRotation`) (* DeltaSeconds (`self.rotateSpeed`)))))

(fn `UserConstructionScript`)