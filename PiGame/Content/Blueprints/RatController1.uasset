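; Player-controlled rat that runs forward each tick and steers around the world X axis, like moving around a tube.
; Horizontal input rotates its location about that axis, and roll is derived from the resulting Y/Z angle.
; Gravity derives from the direction to the axis, but absolute-then-negate keeps every component non-positive.
; A trace along local down gates the jump force; debug prints remain, and helper RotateAround is unused here.
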(event `self.ReceiveTick`
  (params (DeltaSeconds :type "Float (single-precision)"))
  (bind _returnvalue (`self.K2_GetActorLocation`))
  (bind _returnvalue_2 (`self.K2_GetActorLocation`))
  (bind _returnvalue_3 (`KismetMathLibrary.MakeVector` (.x _returnvalue)))
  (bind _returnvalue_4 (`KismetMathLibrary.RotateAngleAxis` _returnvalue (* (`self.rotateSpeed`) (`self.GetInputAxisValue`)) _returnvalue_3))
  (bind _returnvalue_5 (* (`KismetMathLibrary.Vector_GetAbs` (* (`KismetMathLibrary.Normal` (- _returnvalue_3 _returnvalue_4)) (`self.gravityStrength`))) -1.0))
  (bind (_outhit _returnvalue_6) (`KismetSystemLibrary.LineTraceSingle` _returnvalue_2 (+ _returnvalue_2 (* (`self.GetActorUpVector`) -100.0)) "TraceTypeQuery1" true))
  (bind _output_get (set `self.isGrounded` _returnvalue_6))
  (`KismetSystemLibrary.PrintString` (`KismetStringLibrary.Conv_BoolToString` _output_get))
  (`self.K2_AddActorLocalOffset` (* (`self.GetActorForwardVector`) (`self.moveSpeed`)) true)
  (`self.K2_SetActorLocation` _returnvalue_4 true)
  (`self.K2_SetActorRotation` (`KismetMathLibrary.MakeRotator` (* (+ (`KismetMathLibrary.DegAtan2` (.z _returnvalue_4) (.y _returnvalue_4)) 90.0) -1.0)))
  (`PrimitiveComponent.AddForce` (`self.CapsuleCollider`) _returnvalue_5 "None" true)
  (`KismetSystemLibrary.PrintString` (`KismetStringLibrary.Conv_VectorToString` _returnvalue_5)))

(event `InputAction|Jump`
  (params (Key :type "Key Structure"))
  (:`Pressed`
    (if (`self.isGrounded`)
      (`PrimitiveComponent.AddForce` (`self.CapsuleCollider`) (* (`self.GetActorUpVector`) (`self.jumpspeed`)) "None" true))))

(fn `RotateAround`
  (params (Center :type "Vector Structure") (Rotation :type "Rotator Structure") (Distance :type "Float (double-precision)"))
  (returns (`Out Point` :type "Vector Structure"))
  (return (+ Center (* (`KismetMathLibrary.GetForwardVector` Rotation) Distance))))

(fn `UserConstructionScript`)