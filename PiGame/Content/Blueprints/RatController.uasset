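; RatController is an actor that moves continuously and rolls in response to a horizontal value, apparently as a rat controller.
; Each Tick it adds an unswept local offset of its forward vector scaled by MoveSpeed, although that vector is in world space.
; It then combines its rotation with a roll from RotateSpeed and the negated horizontal value.
; Neither movement nor rotation scales by delta time, so both depend on frame rate.
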(event `self.ReceiveTick`
  (params (DeltaSeconds :type "Float (single-precision)"))
  (`self.K2_AddActorLocalOffset` (* (`self.GetActorForwardVector`) (`self.moveSpeed`)))
  (`self.K2_SetActorRotation` (`KismetMathLibrary.ComposeRotators` (`self.K2_GetActorRotation`) (* (`KismetMathLibrary.MakeRotator` (`self.rotateSpeed`)) (* (`self.GetInputAxisValue`) -1.0)))))

(fn `UserConstructionScript`)