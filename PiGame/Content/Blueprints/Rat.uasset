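; Rat actor that runs forward and circles around the world X axis with the Horizontal input, as if inside or around a tube.
; Each Tick it adds a forward offset by MoveSpeed, then rotates its location around that axis by TurnSpeed times input.
; Roll is derived from the Y/Z angle so the rat stays aligned to the circle.
; Movement uses neither sweep nor delta-time scaling.
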(event `self.ReceiveTick`
  (params (DeltaSeconds :type "Float (single-precision)"))
  (bind _returnvalue (`self.K2_GetActorLocation`))
  (bind _returnvalue_2 (`KismetMathLibrary.RotateAngleAxis` _returnvalue (* (`self.turnSpeed`) (`self.GetInputAxisValue`)) (`KismetMathLibrary.MakeVector` (.x _returnvalue))))
  (`self.K2_AddActorLocalOffset` (* (`self.GetActorForwardVector`) (`self.moveSpeed`)))
  (`self.K2_SetActorLocation` _returnvalue_2)
  (`self.K2_SetActorRotation` (`KismetMathLibrary.MakeRotator` (* (+ (`KismetMathLibrary.DegAtan2` (.z _returnvalue_2) (.y _returnvalue_2)) 90.0) -1.0))))

(fn `UserConstructionScript`)